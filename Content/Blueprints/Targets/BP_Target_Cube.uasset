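; BP_Target_Cube is a shootable target that turns its cube green when it takes any damage.
; If flagged IsRestart, the hit reloads MainMap.
; If flagged IsVisibleTarget, it casts its Platform reference to MovingPlatform and sets IsMoving to start that platform.
; All logic runs from the AnyDamage event, with no guard against repeated hits.
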(event EventBeginPlay
  (|CallParentFunction) ; This node is disabled and will not be called.\nDrag off pins to build functionality.
)

(event Collision|EventActorBeginOverlap
  (params (OtherActor :type Actor%20Object%20Reference))
  (|CallParentFunction OtherActor) ; This node is disabled and will not be called.\nDrag off pins to build functionality.
)

(event EventTick
  (params (DeltaSeconds :type Float%20%28single-precision%29))
  (|CallParentFunction DeltaSeconds) ; This node is disabled and will not be called.\nDrag off pins to build functionality.
)

(event Game|Damage|EventAnyDamage
  (params (Damage :type Float%20%28single-precision%29) (DamageType :type Damage%20Type%20Object%20Reference) (InstigatedBy :type Controller%20Object%20Reference) (DamageCauser :type Actor%20Object%20Reference))
  (Rendering|Material|SetMaterial (Variables|Default|GetCube) 0 "/Game/Materials/TargetMaterials/M_Targ_Green.M_Targ_Green")
  (Utilities|FlowControl|Sequence
    (:then_0
      (if (Variables|Default|GetIsRestart)
        (Game|OpenLevel(byName) "MainMap")))
    (:then_1
      (if (Variables|Default|GetIsVisibleTarget)
        (bind _asmoving_platform (Utilities|Casting|CastToMovingPlatform (Variables|Default|GetPlatform)))
        (Variables|/Game/Blueprints/Targets/MovingPlatform.MovingPlatform_C|SetIsMoving _asmoving_platform true)))))

(fn ConstructionScript
  (|CallParentFunction))